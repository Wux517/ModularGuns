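; Health component that gives its owning actor health, a screen-space health bar above it, and timed respawning.
; BeginPlay creates the bar widget component, and Tick updates its fill every frame.
; DealDamage scales damage by a multiplier and Armor (higher Armor increases damage), triggering training-dummy hit or kill effects through casts on the owner.
; At zero health the owner is hidden, not destroyed, until a timer restores health and visibility.
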(event Custom|DealDamage
  (params (Damage :type Float%20%28double-precision%29) (HitComponent :type Actor%20Component%20Object%20Reference))
  (bind _output_get (Variables|Default|SetCurrentHealth (- (Variables|Default|GetCurrentHealth) (* (* (* Damage 3.0) (Variables|Default|GetDamageMultiplier)) (+ (Variables|Default|GetArmor) 1.0)))))
  (if (<= _output_get 0.0)
    (Rendering|SetActorHiddenInGame (Components|GetOwner) true)
    (Utilities|Time|SetTimerbyEvent (delegate Custom|Respawn) (Variables|Default|GetRespawnTimer))
    (bind _asbpc_training_dummy (Utilities|Casting|CastToBPC_TrainingDummy (Components|GetOwner)))
    (Default|PlayKillEffect _asbpc_training_dummy)
    (else
      (bind _asbpc_training_dummy_2 (Utilities|Casting|CastToBPC_TrainingDummy (Components|GetOwner)))
      (Default|PlayHitEffect _asbpc_training_dummy_2))))

(event Custom|Respawn
  (Variables|Default|SetCurrentHealth (Variables|Default|GetMaxHealth))
  (Rendering|SetActorHiddenInGame (Components|GetOwner) false))

(event EventBeginPlay
  (bind _returnvalue (UserInterface|CreateWidget "/Game/Blueprints/UI/WBP_HealthBar.WBP_HealthBar_C"))
  (Variables|Default|SetHealthBatWidget _returnvalue)
  (Variables|Default|SetCurrentHealth (Variables|Default|GetMaxHealth))
  (bind _returnvalue_2 (Game|AddComponentbyClass (Components|GetOwner) "/Script/UMG.WidgetComponent" false (Math|Transform|MakeTransform "0.000000,0.000000,200.000000" "0, 0, 0" "1.000000,1.000000,1.000000")))
  (Class|WidgetComponent|SetWidgetSpace _returnvalue_2 "Screen")
  (Class|WidgetComponent|SetDrawSize _returnvalue_2 "(X=100.000000,Y=15.000000)")
  (UserInterface|SetWidget _returnvalue_2 (Variables|Default|GetHealthBatWidget)))

(event EventTick
  (params (DeltaSeconds :type Float%20%28single-precision%29))
  (Progress|SetPercent (Variables|/Game/Blueprints/UI/WBP_HealthBar.WBP_HealthBar_C|GetProgressBar_35 (Variables|Default|GetHealthBatWidget)) (/ (Variables|Default|GetCurrentHealth) (Variables|Default|GetMaxHealth))))