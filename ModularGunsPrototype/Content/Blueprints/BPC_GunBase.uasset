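; Base gun component that attaches to the first-person character's grip socket, adds weapon input and creates a crosshair.
; Shoot input runs single, burst or automatic fire, spawning projectiles in a spread cone and passing them a camera-trace aim direction.
; Tick widens spread and crosshair with player speed, and while firing kicks control rotation using a timer's elapsed time to ramp recoil.
; Barrel and stock modifiers set stability, velocity and recoil control.
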(event Custom|Setting%20Variables
  (bind _modifiers (Variables|Modifyers|GetModifiers))
  (Variables|Modifyers|SetForce (* (Variables|Modifyers|GetForce) (Variables|Modifyers|GetVelocity)))
  (Variables|Default|SetStartSpreadAngle (Variables|Modifyers|GetSpreadAngle))
  (Utilities|FlowControl|Sequence
    (:then_0
      (CallFunction|SettingBarrelVar (.barrel _modifiers)))
    (:then_1
      (CallFunction|SettingStockVar (.stock _modifiers)))))

(event Input|EnhancedActionEvents|EnhancedInputActionIA_Shoot
  (params (ActionValue :type Boolean) (ElapsedSeconds :type Float%20%28double-precision%29) (TriggeredSeconds :type Float%20%28double-precision%29) (InputAction :type Input%20Action%20Object%20Reference :default "/Game/FirstPerson/Input/Actions/IA_Shoot.IA_Shoot"))
  (:Triggered
    (if (Variables|Default|GetcanFire?)
      (Utilities|FlowControl|DoOnce false :!label _label
        (:Completed
          (Variables|Default|SetisFiring? true)
          (CallFunction|RecoilStart)
          (switch Utilities|FlowControl|Switch|SwitchonE_FireModes (.firemode (Variables|Modifyers|GetModifiers))
            (:NewEnumerator0
              (Utilities|SingleFire))
            (:NewEnumerator1
              (Utilities|BurstFire))
            (:NewEnumerator2
              (Utilities|AutomaticFire)))))))
  (:Completed
    (Variables|Default|SetisFiring? false)
    (goto _label Reset)))

(event EventTick
  (params (DeltaSeconds :type Float%20%28single-precision%29))
  (CallFunction|CalculateSpread)
  (if (Variables|Default|GetisFiring?)
    (CallFunction|Recoil)
    (else
      (CallFunction|RecoilStop))))

(event EventBeginPlay
  (CallFunction|SettingVariables)
  (bind _asbp_first_person_character (Utilities|Casting|CastToBP_FirstPersonCharacter (Components|GetOwner)))
  (Variables|Default|SetFirst%20PersonCharacter _asbp_first_person_character)
  (Transformation|AttachComponentToComponent (Variables|/Game/FirstPerson/Blueprints/BP_FirstPersonCharacter.BP_FirstPersonCharacter_C|GetFirstPersonMesh _asbp_first_person_character) "GripPoint" "KeepRelative" "KeepRelative" "KeepRelative" true)
  (Variables|/Game/FirstPerson/Blueprints/BP_FirstPersonCharacter.BP_FirstPersonCharacter_C|SetbHasRifle (Variables|Default|GetFirst%20PersonCharacter) true)
  (bind _asplayer_controller (Utilities|Casting|CastToPlayerController (Pawn|GetController (Variables|Default|GetFirst%20PersonCharacter))))
  (Utilities|IsValid (PlayerController|LocalPlayerSubsystems|GetEnhancedInputLocalPlayerSubsystem _asplayer_controller)
    (:Is%20Valid
      (Input|AddMappingContext (PlayerController|LocalPlayerSubsystems|GetEnhancedInputLocalPlayerSubsystem _asplayer_controller) "/Game/FirstPerson/Input/IMC_Weapons.IMC_Weapons" 1 "(bIgnoreAllPressedKeysUntilRelease=True,bForceImmediately=False)")
      (bind _returnvalue (UserInterface|CreateWidget "/Game/Blueprints/Widgets/WBP_Crosshair.WBP_Crosshair_C"))
      (bind _output_get (Variables|Default|SetCrosshair _returnvalue))
      (UserInterface|Viewport|AddtoViewport _output_get 0))))

(fn Fire
  (bind _returnvalue (Transformation|GetSocketLocation "Ammo"))
  (bind _projectileoffset (Variables|Default|GetProjectileOffset))
  (bind _returnvalue_2 (+ _returnvalue _projectileoffset))
  (Variables|Default|SetcanFire? false)
  (Utilities|Time|SetTimerbyFunctionName 0 "ShotCooldown" (Variables|Modifyers|GetCooldown))
  (Game|Feedback|ClientStartCameraShake (Game|GetPlayerController 0) "/Game/Blueprints/CameraShake/BP_RecoilCameraShake.BP_RecoilCameraShake_C" 1.0 "CameraLocal" "0, 0, 0")
  (if (Variables|Modifyers|GetSpreadSpawner?)
    (for _index (range 1 (Variables|Modifyers|GetProjectile%20Amount))
      (bind _returnvalue_3 (Game|SpawnActorfromClass (Variables|Default|GetClass) (Math|Transform|MakeTransform _returnvalue_2 (Math|Rotator|MakeRotfromX (Math|Random|RandomUnitVectorinConeinDegrees (Transformation|GetActorForwardVector (Game|GetPlayerCameraManager 0)) (Variables|Modifyers|GetSpreadAngle))) "1.000000,1.000000,1.000000") "Undefined" "SelectDefaultAtRuntime" 0 0))
      (Audio|SpawnSoundatLocation "/Game/FPWeapon/Audio/FirstPersonTemplateWeaponFire02.FirstPersonTemplateWeaponFire02" _returnvalue_2 "0, 0, 0" 1.0 1.0 0.0 0 0)
      (bind _forwardvectortotarget (CallFunction|GetTargetPos _returnvalue_2))
      (Class|BPIFire|Fire(Message) _returnvalue_3 (Variables|Modifyers|GetForce) _forwardvectortotarget))
    (else
      (bind _returnvalue_4 (Game|SpawnActorfromClass (Variables|Default|GetClass) (Math|Transform|MakeTransform _returnvalue_2 (Math|Rotator|MakeRotfromX (Math|Random|RandomUnitVectorinConeinDegrees (Transformation|GetActorForwardVector (Game|GetPlayerCameraManager 0)) (Variables|Modifyers|GetSpreadAngle))) "1.000000,1.000000,1.000000") "Undefined" "SelectDefaultAtRuntime" 0 0))
      (Audio|SpawnSoundatLocation "/Game/FPWeapon/Audio/FirstPersonTemplateWeaponFire02.FirstPersonTemplateWeaponFire02" _returnvalue_2 "0, 0, 0" 1.0 1.0 0.0 0 0)
      (bind _forwardvectortotarget_2 (CallFunction|GetTargetPos _returnvalue_2))
      (Class|BPIFire|Fire(Message) _returnvalue_4 (Variables|Modifyers|GetForce) _forwardvectortotarget_2))))

(fn RecoilStart
  (bind _returnvalue (Utilities|Time|SetTimerbyFunctionName 0 "Recoil" 1e+01))
  (Variables|Default|SetElapsedTimeRecoil _returnvalue)
  (Variables|Default|SetStartingControlRotation (Pawn|GetControlRotation (Game|GetPlayerController 0) :!class /Script/Engine.Controller)))

(fn RecoilStop
  (Utilities|Time|ClearandInvalidateTimerbyHandle (Variables|Default|GetElapsedTimeRecoil))
  (if (Variables|Default|GetisRecovering)
    _))

(fn RecoveryStartFunction
  (bind _returnvalue (Game|GetPlayerState 0))
  (bind _returnvalue_2 (Game|GetPlayerController _returnvalue))
  (bind _returnvalue_3 (Pawn|GetControlRotation _returnvalue_2 :!class /Script/Engine.Controller))
  (Pawn|SetControlRotation (Game|GetPlayerController (Game|GetPlayerState 0)) (Math|Rotator|MakeRotator (.roll _returnvalue_3) (- (.pitch _returnvalue_3) (Variables|Default|GetAddedRecoilY)) (- (.yaw _returnvalue_3) (Variables|Default|GetAddedRecoilZ)))))

(fn Recoil
  (bind _returnvalue (Game|GetPlayerState 0))
  (bind _elapsedtimerecoil (Variables|Default|GetElapsedTimeRecoil))
  (bind _force (Variables|Modifyers|GetForce))
  (bind _minrecoily (Variables|Default|GetMinRecoilY))
  (bind _recoilcontrol (Variables|Modifyers|GetRecoilControl))
  (bind _recoilcontrol_2 (Variables|Modifyers|GetRecoilControl))
  (bind _maxrecoily (Variables|Default|GetMaxRecoilY))
  (bind _recoilexponentialrate (Variables|Default|GetRecoilExponentialRate))
  (bind _returnvalue_2 (Class|KismetSystemLibrary|GetTimerElapsedTimeHandle _elapsedtimerecoil))
  (bind _returnvalue_3 (Game|GetPlayerController _returnvalue))
  (bind _returnvalue_4 (* _maxrecoily _recoilcontrol))
  (bind _returnvalue_5 (* _recoilexponentialrate 1e-05))
  (bind _returnvalue_6 (/ _minrecoily _recoilcontrol_2))
  (bind _returnvalue_7 (Pawn|GetControlRotation _returnvalue_3 :!class /Script/Engine.Controller))
  (bind _returnvalue_8 (* _returnvalue_2 _returnvalue_5))
  (bind _returnvalue_9 (* _force _returnvalue_8))
  (bind _returnvalue_10 (Math|Float|Clamp(Float) _returnvalue_9 _returnvalue_6 _returnvalue_4))
  (bind _returnvalue_11 (- _returnvalue_10 0.05))
  (bind _returnvalue_12 (+ _returnvalue_10 0.05))
  (bind _returnvalue_13 (Math|Random|RandomFloatinRange _returnvalue_11 _returnvalue_12))
  (Variables|Default|SetStartingControlRotation (Pawn|GetControlRotation (Game|GetPlayerController (Game|GetPlayerState 0)) :!class /Script/Engine.Controller))
  (bind _output_get (Variables|Default|SetRecoilControlRotation (Math|Rotator|MakeRotator (.roll _returnvalue_7) (+ (.pitch _returnvalue_7) _returnvalue_13) (+ (.yaw _returnvalue_7) (Math|Float|Clamp(Float) _returnvalue_13 0.0 (* (Variables|Default|GetMaxRecoilZ) (Variables|Modifyers|GetRecoilControl)))))))
  (Pawn|SetControlRotation (Game|GetPlayerController (Game|GetPlayerState 0)) _output_get)
  (Variables|Default|SetisRecovering true))

(fn CalculateSpread
  (bind _returnvalue (Game|GetPlayerCharacter 0))
  (Variables|Modifyers|SetSpreadAngle (* (Math|Float|Clamp(Float) (+ (Variables|Default|GetStartSpreadAngle) (/ (Math|Vector|VectorLength (Transformation|GetVelocity _returnvalue)) (Class|MovementComponent|GetMaxSpeed (Variables|/Script/Engine.Character|GetCharacterMovement _returnvalue)))) (Variables|Default|GetStartSpreadAngle) (+ (Variables|Default|GetStartSpreadAngle) 2.0)) (Variables|Modifyers|GetStability)))
  (CallFunction|UpdateCrosshair)
  (return))

(fn GetTargetPos
  (params (Origin :type Vector))
  (bind _first_personcharacter (Variables|Default|GetFirst%20PersonCharacter))
  (bind _firstpersoncamera (Variables|/Game/FirstPerson/Blueprints/BP_FirstPersonCharacter.BP_FirstPersonCharacter_C|GetFirstPersonCamera _first_personcharacter))
  (bind _returnvalue (Transformation|GetWorldLocation _firstpersoncamera))
  (bind _outhit (Collision|LineTraceByChannel _returnvalue (+ _returnvalue (* (Math|Vector|GetForwardVector _firstpersoncamera) 1e+04)) "TraceTypeQuery1" false 0 "Persistent"))
  (return (Math|Vector|Normalize (- (.ImpactPoint (Collision|BreakHitResult _outhit)) Origin))))

(fn UpdateCrosshair
  (Utilities|FlowControl|Sequence
    (:then_0
      (Class|Widget|SetRenderTranslation (Variables|/Game/Blueprints/Widgets/WBP_Crosshair.WBP_Crosshair_C|GetBottom (Variables|Default|GetCrosshair)) (Math|Vector2D|MakeVector2D 0.0 (* (Variables|Modifyers|GetSpreadAngle) 1e+01))))
    (:then_1
      (Class|Widget|SetRenderTranslation (Variables|/Game/Blueprints/Widgets/WBP_Crosshair.WBP_Crosshair_C|GetTop (Variables|Default|GetCrosshair)) (Math|Vector2D|MakeVector2D 0.0 (* (Variables|Modifyers|GetSpreadAngle) -1e+01))))
    (:then_2
      (Class|Widget|SetRenderTranslation (Variables|/Game/Blueprints/Widgets/WBP_Crosshair.WBP_Crosshair_C|GetRight (Variables|Default|GetCrosshair)) (Math|Vector2D|MakeVector2D (* (Variables|Modifyers|GetSpreadAngle) 1e+01) 0.0)))
    (:then_3
      (Class|Widget|SetRenderTranslation (Variables|/Game/Blueprints/Widgets/WBP_Crosshair.WBP_Crosshair_C|GetLeft (Variables|Default|GetCrosshair)) (Math|Vector2D|MakeVector2D (* (Variables|Modifyers|GetSpreadAngle) -1e+01) 0.0)))))

(fn SettingBarrelVar
  (params (Selection :type E_Barrels%20Enum :default "NewEnumerator0"))
  ;[1 1 1] Barrels
  (switch Utilities|FlowControl|Switch|SwitchonE_Barrels Selection
    (:NewEnumerator0
      (Variables|Modifyers|SetStability 0.0)
      (Variables|Modifyers|SetVelocity 1.0))
    (:NewEnumerator1
      (Variables|Modifyers|SetStability 0.5)
      (Variables|Modifyers|SetVelocity 1.0))
    (:NewEnumerator2
      (Variables|Modifyers|SetStability 1.0)
      (Variables|Modifyers|SetVelocity 1.1))
    (:NewEnumerator3
      (Variables|Modifyers|SetStability 1.5)
      (Variables|Modifyers|SetVelocity 1.25))))

(fn SettingStockVar
  (params (Selection :type E_Stock%20Enum :default "NewEnumerator0"))
  ;[1 1 1] Stocks
  (switch Utilities|FlowControl|Switch|SwitchonE_Stock Selection
    (:NewEnumerator0
      (Variables|Modifyers|SetRecoilControl 5.0))
    (:NewEnumerator1
      (Variables|Modifyers|SetRecoilControl 3.0))
    (:NewEnumerator2
      (Variables|Modifyers|SetRecoilControl 1.0))))

(fn ShotCooldown
  (Variables|Default|SetcanFire? true))