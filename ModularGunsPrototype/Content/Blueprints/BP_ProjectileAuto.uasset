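; BP_ProjectileAuto is a physics-driven projectile that damages and pushes what it hits.
; Fire records the start location and applies force to the capsule, scaled by Force over Mass along the TargetLocation vector.
; On impact, average velocity from distance over lifetime times Mass gives a momentum that becomes an impulse on physics-simulating components.
; The capsule hit sends scaled momentum magnitude as damage through ChangeHealthMessage, then destroys the projectile.
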(event OnComponentHit(Capsule)
  (params (HitComponent :type Primitive%20Component%20Object%20Reference) (OtherActor :type Actor%20Object%20Reference) (OtherComp :type Primitive%20Component%20Object%20Reference) (NormalImpulse :type Vector :default "0, 0, 0") (Hit :type Hit%20Result%20Structure%20%28by%20ref%29))
  (Utilities|IsValid OtherActor
    (:Is%20Valid
      (Class|BPIHealth|ChangeHealth(Message) OtherActor (* (/ (Math|Vector|VectorLength (* (Variables|Default|GetMass) (/ (- (Variables|Default|GetFinalLocation) (Variables|Default|GetInitialLocation)) (Actor|GetGameTimeSinceCreation)))) 1e+02) 0.5) OtherComp)
      (Actor|DestroyActor))))

(event EventBeginPlay)

(event Collision|EventActorBeginOverlap
  (params (OtherActor :type Actor%20Object%20Reference)))

(event Collision|EventHit
  (params (MyComp :type Primitive%20Component%20Object%20Reference) (Other :type Actor%20Object%20Reference) (OtherComp :type Primitive%20Component%20Object%20Reference) (bSelfMoved :type Boolean) (HitLocation :type Vector :default "0, 0, 0") (HitNormal :type Vector :default "0, 0, 0") (NormalImpulse :type Vector :default "0, 0, 0") (Hit :type Hit%20Result%20Structure%20%28by%20ref%29))
  (Variables|Default|SetFinalLocation HitLocation)
  (Utilities|IsValid OtherComp
    (:Is%20Valid
      (if (Physics|IsSimulatingPhysics OtherComp "None")
        (Physics|AddImpulseatLocation OtherComp (* (Variables|Default|GetMass) (/ (- (Variables|Default|GetFinalLocation) (Variables|Default|GetInitialLocation)) (Actor|GetGameTimeSinceCreation))) (Transformation|GetActorLocation) "None")))))

(event EventFire
  (params (Force :type Float%20%28double-precision%29) (TargetLocation :type Vector :default "0, 0, 0"))
  (Variables|Default|SetInitialLocation (Transformation|GetActorLocation))
  (Physics|AddForce (Variables|Default|GetCapsule) (* TargetLocation (/ Force (Variables|Default|GetMass))) "None" false))

(fn ConstructionScript)