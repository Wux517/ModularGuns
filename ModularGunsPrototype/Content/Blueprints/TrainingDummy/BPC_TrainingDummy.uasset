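; Training dummy actor that takes damage with critical and limb modifiers and can optionally be repositioned.
; ChangeHealth forwards damage and the hit component to BPCHealth.
; Overlaps on the head, arm and leg colliders set that component's DamageMultiplier to its critical or limb value, with no reset here.
; When ShouldMove is set, BeginPlay makes a single lerped jump between two locations by TimeToMove, without animating over time.
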(event OnComponentBeginOverlap(HeadCollision)
  (params (OverlappedComponent :type Primitive%20Component%20Object%20Reference) (OtherActor :type Actor%20Object%20Reference) (OtherComp :type Primitive%20Component%20Object%20Reference) (OtherBodyIndex :type Integer) (bFromSweep :type Boolean) (SweepResult :type Hit%20Result%20Structure%20%28by%20ref%29))
  (bind _bpc_health (Variables|Default|GetBPC_Health))
  (Variables|/Game/Blueprints/BPC_Health.BPC_Health_C|SetDamageMultiplier _bpc_health (Variables|/Game/Blueprints/BPC_Health.BPC_Health_C|GetCriticalDamageMultiplier _bpc_health)))

(event OnComponentBeginOverlap(Legs)
  (params (OverlappedComponent :type Primitive%20Component%20Object%20Reference) (OtherActor :type Actor%20Object%20Reference) (OtherComp :type Primitive%20Component%20Object%20Reference) (OtherBodyIndex :type Integer) (bFromSweep :type Boolean) (SweepResult :type Hit%20Result%20Structure%20%28by%20ref%29))
  (bind _bpc_health (Variables|Default|GetBPC_Health))
  (Variables|/Game/Blueprints/BPC_Health.BPC_Health_C|SetDamageMultiplier _bpc_health (Variables|/Game/Blueprints/BPC_Health.BPC_Health_C|GetLimbDamageMultiplier _bpc_health)))

(event OnComponentBeginOverlap(rArm)
  (params (OverlappedComponent :type Primitive%20Component%20Object%20Reference) (OtherActor :type Actor%20Object%20Reference) (OtherComp :type Primitive%20Component%20Object%20Reference) (OtherBodyIndex :type Integer) (bFromSweep :type Boolean) (SweepResult :type Hit%20Result%20Structure%20%28by%20ref%29))
  (bind _bpc_health (Variables|Default|GetBPC_Health))
  (Variables|/Game/Blueprints/BPC_Health.BPC_Health_C|SetDamageMultiplier _bpc_health (Variables|/Game/Blueprints/BPC_Health.BPC_Health_C|GetLimbDamageMultiplier _bpc_health)))

(event OnComponentBeginOverlap(lArm)
  (params (OverlappedComponent :type Primitive%20Component%20Object%20Reference) (OtherActor :type Actor%20Object%20Reference) (OtherComp :type Primitive%20Component%20Object%20Reference) (OtherBodyIndex :type Integer) (bFromSweep :type Boolean) (SweepResult :type Hit%20Result%20Structure%20%28by%20ref%29))
  (bind _bpc_health (Variables|Default|GetBPC_Health))
  (Variables|/Game/Blueprints/BPC_Health.BPC_Health_C|SetDamageMultiplier _bpc_health (Variables|/Game/Blueprints/BPC_Health.BPC_Health_C|GetLimbDamageMultiplier _bpc_health)))

(event EventBeginPlay
  (if (Variables|Default|GetShouldMove?)
    (if (> (Variables|Default|GetCurrentPosition) 0)
      (Transformation|SetActorLocation (Math|Vector|Lerp(Vector) (Variables|Default|GetLocation1) (Variables|Default|GetLocation2) (Variables|Default|GetTimeToMove)) false false)
      (Variables|Default|SetCurrentPosition 0)
      (else
        (bind _output_get (Variables|Default|SetLocation2 (Transformation|GetActorLocation)))
        (Transformation|SetActorRelativeLocation (Math|Vector|Lerp(Vector) _output_get (Variables|Default|GetLocation1) (Variables|Default|GetTimeToMove)))
        (Variables|Default|SetCurrentPosition 1)))))

(event Collision|EventActorBeginOverlap
  (params (OtherActor :type Actor%20Object%20Reference)))

(event EventTick
  (params (DeltaSeconds :type Float%20%28single-precision%29)))

(event EventChangeHealth
  (params (Damage :type Float%20%28double-precision%29) (HitComponent :type Actor%20Component%20Object%20Reference))
  (Default|DealDamage (Variables|Default|GetBPC_Health) Damage HitComponent))

(fn ConstructionScript)